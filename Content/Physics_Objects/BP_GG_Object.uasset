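; Physics object that the player can rotate with per-axis inputs while the character's physics handle is active.
; BeginPlay caches the BP_PlayerCharacter; each rotate press sets a constant rate on the RotatingMovement component and any release zeroes it.
; The check reads only the character's PhysicsHandleActive flag on press, not whether this particular object is the one held.
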(event `self.ReceiveBeginPlay`
  (bind _asbp_player_character (cast `/Game/Player/BP_PlayerCharacter` (`GameplayStatics.GetPlayerCharacter` 0)))
  (set `self.As BP Player Character` _asbp_player_character))

(event `InputAction|RotateObjectZ`
  (params (Key :type "Key Structure"))
  (bind _rotatingmovement (`self.RotatingMovement`))
  ;[1 1 1] Rotate Held Object
  ;;[1 1 1] Rotate Z Axis
  (:`Pressed`
    (if (`/Game/Player/BP_PlayerCharacter.physicsHandleActive` (`self.As BP Player Character`))
      (set `RotatingMovementComponent.RotationRate` (struct :`Yaw` 20.0) _rotatingmovement)))
  (:`Released`
    (set `RotatingMovementComponent.RotationRate` (struct) _rotatingmovement)))

(event `InputAction|RotateObjectX`
  (params (Key :type "Key Structure"))
  (bind _rotatingmovement (`self.RotatingMovement`))
  ;[1 1 1] Rotate Held Object
  ;;[1 1 1] Rotate X Axis
  (:`Pressed`
    (if (`/Game/Player/BP_PlayerCharacter.physicsHandleActive` (`self.As BP Player Character`))
      (set `RotatingMovementComponent.RotationRate` (struct :`Roll` 20.0) _rotatingmovement)))
  (:`Released`
    (set `RotatingMovementComponent.RotationRate` (struct) _rotatingmovement)))

(event `InputAction|RotateObjectY`
  (params (Key :type "Key Structure"))
  (bind _rotatingmovement (`self.RotatingMovement`))
  ;[1 1 1] Rotate Held Object
  ;;[1 1 1] Rotate Y Axis
  (:`Pressed`
    (if (`/Game/Player/BP_PlayerCharacter.physicsHandleActive` (`self.As BP Player Character`))
      (set `RotatingMovementComponent.RotationRate` (struct :`Pitch` 20.0) _rotatingmovement)))
  (:`Released`
    (set `RotatingMovementComponent.RotationRate` (struct) _rotatingmovement)))

(fn `UserConstructionScript`)