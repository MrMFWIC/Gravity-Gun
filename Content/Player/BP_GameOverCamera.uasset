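; Game-over camera actor that takes over the player's view and keeps aimed above the BP_Target actor.
; BeginPlay looks up the target, and Tick rotates the camera toward a point raised above it.
; SwapCamera blends the view to this actor through the player controller, then starts CameraZoom.
; The zoom timeline cumulatively offsets the camera's world position each update and drives its field of view.
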(event `self.ReceiveTick`
  (params (DeltaSeconds :type "Float (single-precision)"))
  (`self.Camera Focus` (`self.K2_GetActorLocation` (`self.TargetRef`))))

(event `self.ReceiveBeginPlay`
  (bind _asbp_target (castclass `/Game/Objectives/BP_Target` "/Game/Objectives/BP_Target.BP_Target_C"))
  (bind _returnvalue (`GameplayStatics.GetActorOfClass` _asbp_target))
  (set `self.TargetRef` _returnvalue))

(event `Swap Camera`
  (bind _asbp_player_character (cast `/Game/Player/BP_PlayerCharacter` (`GameplayStatics.GetPlayerCharacter` 0)))
  (`/Game/Player/BP_PlayerController.SwitchCamera` (`/Game/Player/BP_PlayerCharacter.As BP Player Controller` _asbp_player_character) self (`self.Blend Time`))
  (`self.Camera Zoom`))

(event `Camera Focus`
  (params (Target :type "Vector Structure"))
  (bind _camera (`self.Camera`))
  (set `CameraComponent.bUsePawnControlRotation` false _camera)
  (`SceneComponent.K2_SetWorldRotation` _camera (`KismetMathLibrary.FindLookAtRotation` (`SceneComponent.K2_GetComponentLocation` _camera) (+ Target (0.0 0.0 1400.0))) false false))

(event `Camera Zoom`
  (bind _camera (`self.Camera`))
  (bind (_direction _transform_changes _camera_fov) (`Timeline|Timeline`)
    (:`Update`
      (`SceneComponent.K2_SetWorldLocation` _camera (+ (`SceneComponent.K2_GetComponentLocation` _camera) (`KismetMathLibrary.MakeVector` (.x _transform_changes) (* (.y _transform_changes) -1.0) (.z _transform_changes))) false false)
      (`CameraComponent.SetFieldOfView` _camera (* _camera_fov 90.0)))))

(fn `UserConstructionScript`)