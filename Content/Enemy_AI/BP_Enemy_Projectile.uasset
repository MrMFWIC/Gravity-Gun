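; Enemy projectile Blueprint that launches itself at the player when it spawns.
; On BeginPlay it applies a fixed-strength physics impulse to its Sphere along the direction to the player's current position, then prints a debug message.
; The aim is set once, with no homing afterward.
; A delayed self-destroy chain exists but is disconnected, so this graph never destroys the projectile.
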(event `self.ReceiveBeginPlay`
  (`PrimitiveComponent.AddImpulse` (`self.Sphere`) (* (`KismetMathLibrary.Normal` (- (`self.K2_GetActorLocation` (`GameplayStatics.GetPlayerCharacter` 0)) (`self.K2_GetActorLocation`))) 25000.0) "None" false)
  (`KismetSystemLibrary.PrintString` "impulse added"))

(fn `UserConstructionScript`)