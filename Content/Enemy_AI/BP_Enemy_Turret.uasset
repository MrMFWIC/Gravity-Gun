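; BP_Enemy_Turret is an enemy turret that turns toward the player and fires projectiles when it sees them.
; Each PawnSensing sighting of BP_PlayerCharacter snaps the actor's rotation to face the player.
; A randomized Delay, which also throttles repeated sightings, precedes a 2D spell-cast cue.
; After a short wind-up, it spawns BP_Enemy_Projectile at the Arrow component's transform.
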(event `self.PawnSensing.OnSeePawn`
  (params (Pawn :type "Pawn Object Reference"))
  (cast `/Game/Player/BP_PlayerCharacter` Pawn)
  (`self.K2_SetActorRotation` (`KismetMathLibrary.FindLookAtRotation` (`self.K2_GetActorLocation`) (`self.K2_GetActorLocation` Pawn)))
  (`KismetSystemLibrary.Delay` (`KismetMathLibrary.RandomFloatInRange` 1.5 4.0))
  (`GameplayStatics.PlaySound2D` "/Game/Audio/SFX/Spell_Cast_Cue.Spell_Cast_Cue" 1.0 1.0 0.0 null null)
  (`KismetSystemLibrary.Delay` 0.4)
  (`|SpawnActorFromClass` "/Game/Enemy_AI/BP_Enemy_Projectile.BP_Enemy_Projectile_C" (`SceneComponent.K2_GetComponentToWorld` (`self.Arrow`)) "Undefined" "OverrideRootScale" null null))

(fn `UserConstructionScript`)