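; BP_Barrier is an objective barrier that removes itself once the blue, red and yellow crystals are all on their pedestals.
; On BeginPlay it finds and caches one actor of each colored pedestal class using GetActorOfClass.
; Its CrystalPlaced event checks each pedestal's crystal-added flag and destroys the barrier when all three are true.
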(event `self.ReceiveBeginPlay`
  (`self.Get Pedastal References`))

(event `Get Pedastal References`
  (bind _returnvalue (`GameplayStatics.GetActorOfClass` "/Game/Objectives/BP_Pedastal_C_Blue.BP_Pedastal_C_Blue_C"))
  (set `self.Blue Pedestal` _returnvalue)
  (bind _returnvalue_2 (`GameplayStatics.GetActorOfClass` "/Game/Objectives/BP_Pedastal_C_Red.BP_Pedastal_C_Red_C"))
  (set `self.Red Pedestal` _returnvalue_2)
  (bind _returnvalue_3 (`GameplayStatics.GetActorOfClass` "/Game/Objectives/BP_Pedastal_C_Yellow.BP_Pedastal_C_Yellow_C"))
  (set `self.Yellow Pedestal` _returnvalue_3))

(event `Crystal Placed`
  (if (and (`/Game/Objectives/BP_Pedastal_C_Blue.BlueCrystalAdded` (`self.Blue Pedestal`)) (`/Game/Objectives/BP_Pedastal_C_Red.RedCrystalAdded` (`self.Red Pedestal`)) (`/Game/Objectives/BP_Pedastal_C_Yellow.YellowCrystalAdded` (`self.Yellow Pedestal`)))
    (`self.K2_DestroyActor`)))

(fn `UserConstructionScript`)