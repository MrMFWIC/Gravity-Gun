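; Red crystal pedestal objective for Level 1 that tracks whether a red crystal is placed on it.
; A Box overlap with BP_GG_Object_Crystal_Red sets RedCrystalAdded, shows the Sphere component and plays a placement sound.
; Any end overlap on the Box clears the flag and hides the Sphere, without checking which actor left.
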(event `self.ReceiveBeginPlay`
  (set `self.RedCrystalAdded` false))

(event `self.Box.OnComponentBeginOverlap`
  (params (OverlappedComponent :type "PrimitiveComponent Object Reference") (OtherActor :type "Actor Object Reference") (OtherComp :type "PrimitiveComponent Object Reference") (OtherBodyIndex :type Integer) (bFromSweep :type Boolean) (SweepResult :type "HitResult Structure (by ref)"))
  (cast `/Game/Physics_Objects/BP_GG_Object_Crystal_Red` OtherActor)
  (if true
    (set `self.RedCrystalAdded` true)
    (`SceneComponent.SetVisibility` (`self.Sphere`) true false)
    (`GameplayStatics.PlaySound2D` "/Game/Audio/SFX/CrystalPlaced_Cue.CrystalPlaced_Cue" 1.0 1.0 0.0 null null)))

(event `self.Box.OnComponentEndOverlap`
  (params (OverlappedComponent :type "PrimitiveComponent Object Reference") (OtherActor :type "Actor Object Reference") (OtherComp :type "PrimitiveComponent Object Reference") (OtherBodyIndex :type Integer))
  (set `self.RedCrystalAdded` false)
  (`SceneComponent.SetVisibility` (`self.Sphere`) false false))

(fn `UserConstructionScript`
  (`parent.UserConstructionScript`))