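; Blue crystal pedestal objective that tells the level's BP_Barrier when a blue crystal sits on it.
; A Box overlap with BP_GG_Object_Crystal_Blue sets BlueCrystalAdded and prints a debug message, while any end overlap clears the flag regardless of actor.
; Tick polls the flag and, while it is set, looks up BP_Barrier with GetActorOfClass and calls CrystalPlaced every frame.
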(event `self.ReceiveBeginPlay`
  (set `self.BlueCrystalAdded` false))

(event `self.ReceiveTick`
  (params (DeltaSeconds :type "Float (single-precision)"))
  (if (`self.BlueCrystalAdded`)
    (bind _returnvalue (`GameplayStatics.GetActorOfClass` "/Game/Objectives/BP_Barrier.BP_Barrier_C"))
    (`/Game/Objectives/BP_Barrier.Crystal Placed` _returnvalue)))

(event `self.Box.OnComponentBeginOverlap`
  (params (OverlappedComponent :type "PrimitiveComponent Object Reference") (OtherActor :type "Actor Object Reference") (OtherComp :type "PrimitiveComponent Object Reference") (OtherBodyIndex :type Integer) (bFromSweep :type Boolean) (SweepResult :type "HitResult Structure (by ref)"))
  (cast `/Game/Physics_Objects/BP_GG_Object_Crystal_Blue` OtherActor)
  (if true
    (set `self.BlueCrystalAdded` true)
    (`KismetSystemLibrary.PrintString` "Blue Crystal Added")))

(event `self.Box.OnComponentEndOverlap`
  (params (OverlappedComponent :type "PrimitiveComponent Object Reference") (OtherActor :type "Actor Object Reference") (OtherComp :type "PrimitiveComponent Object Reference") (OtherBodyIndex :type Integer))
  (set `self.BlueCrystalAdded` false))

(fn `UserConstructionScript`
  (`parent.UserConstructionScript`))