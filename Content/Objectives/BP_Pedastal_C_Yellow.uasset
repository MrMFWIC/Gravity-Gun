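; Yellow crystal pedestal objective that detects a yellow crystal in its box trigger and notifies the barrier.
; A yellow crystal entering the box sets a placed flag and shows the sphere.
; Any actor leaving the box clears the flag and hides the sphere, without a type check.
; While the flag is set, Tick looks up BP_Barrier and calls CrystalPlaced every frame.
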(event `self.ReceiveBeginPlay`
  (set `self.YellowCrystalAdded` false))

(event `self.ReceiveTick`
  (params (DeltaSeconds :type "Float (single-precision)"))
  (if (`self.YellowCrystalAdded`)
    (bind _returnvalue (`GameplayStatics.GetActorOfClass` "/Game/Objectives/BP_Barrier.BP_Barrier_C"))
    (`/Game/Objectives/BP_Barrier.Crystal Placed` _returnvalue)))

(event `self.Box.OnComponentBeginOverlap`
  (params (OverlappedComponent :type "PrimitiveComponent Object Reference") (OtherActor :type "Actor Object Reference") (OtherComp :type "PrimitiveComponent Object Reference") (OtherBodyIndex :type Integer) (bFromSweep :type Boolean) (SweepResult :type "HitResult Structure (by ref)"))
  (cast `/Game/Physics_Objects/BP_GG_Object_Crystal_Yellow` OtherActor)
  (if true
    (set `self.YellowCrystalAdded` true)
    (`SceneComponent.SetVisibility` (`self.Sphere`) true false)))

(event `self.Box.OnComponentEndOverlap`
  (params (OverlappedComponent :type "PrimitiveComponent Object Reference") (OtherActor :type "Actor Object Reference") (OtherComp :type "PrimitiveComponent Object Reference") (OtherBodyIndex :type Integer))
  (set `self.YellowCrystalAdded` false)
  (`SceneComponent.SetVisibility` (`self.Sphere`) false false))

(fn `UserConstructionScript`
  (`parent.UserConstructionScript`))