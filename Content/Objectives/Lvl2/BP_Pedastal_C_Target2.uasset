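; BP_Pedastal_C_Target2 is a Level 2 objective target that registers hits from arrow projectiles.
; It starts with a red sphere visible and TargetHit false.
; When a BP_Projectile_Arrow overlaps its box, it destroys the arrow, swaps to the green sphere, plays the CrystalPlaced cue and sets TargetHit.
; Nothing here resets the target after a hit or reads the flag.
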(event `self.ReceiveBeginPlay`
  (`SceneComponent.SetVisibility` (`self.SphereRed`) true false)
  (`SceneComponent.SetVisibility` (`self.SphereGreen`) false false)
  (set `self.TargetHit` false))

(event `self.Box.OnComponentBeginOverlap`
  (params (OverlappedComponent :type "PrimitiveComponent Object Reference") (OtherActor :type "Actor Object Reference") (OtherComp :type "PrimitiveComponent Object Reference") (OtherBodyIndex :type Integer) (bFromSweep :type Boolean) (SweepResult :type "HitResult Structure (by ref)"))
  (bind _asbp_projectile_arrow (cast `/Game/Objectives/Lvl2/BP_Projectile_Arrow` OtherActor))
  (`self.K2_DestroyActor` _asbp_projectile_arrow)
  (`SceneComponent.SetVisibility` (`self.SphereRed`) false false)
  (`SceneComponent.SetVisibility` (`self.SphereGreen`) true false)
  (`GameplayStatics.PlaySound2D` "/Game/Audio/SFX/CrystalPlaced_Cue.CrystalPlaced_Cue" 1.0 1.0 0.0 null null)
  (set `self.TargetHit` true))

(fn `UserConstructionScript`
  (`parent.UserConstructionScript`))