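; BP_Ballista is a Level 2 objective ballista that the player aims and fires.
; Every tick it reads shot force and input flags from BP_PlayerCharacter, then calls the matching rotate or fire event.
; Rotation moves in one-degree steps within yaw and pitch limits.
; Firing plays a sound, spawns an arrow projectile with a forward impulse scaled by shot force, and uses a DoOnce with delayed reset as cooldown.
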(event `self.ReceiveTick`
  (params (DeltaSeconds :type "Float (single-precision)"))
  ;[1 1 1] Call Events
  (bind _asbp_player_character (cast `/Game/Player/BP_PlayerCharacter` (`GameplayStatics.GetPlayerCharacter` 0)))
  (set `self.Cur Shot Force` (`/Game/Player/BP_PlayerCharacter.CurShotForce` _asbp_player_character))
  (if (`/Game/Player/BP_PlayerCharacter.BallistaFire` _asbp_player_character)
    (`self.Fire`))
  (if (`/Game/Player/BP_PlayerCharacter.UpKeyPressed` _asbp_player_character)
    (`self.RotateUp`))
  (if (`/Game/Player/BP_PlayerCharacter.DownKeyPressed` _asbp_player_character)
    (`self.RotateDown`))
  (if (`/Game/Player/BP_PlayerCharacter.LeftKeyPressed` _asbp_player_character)
    (`self.RotateLeft`))
  (if (`/Game/Player/BP_PlayerCharacter.RightKeyPressed` _asbp_player_character)
    (`self.RotateRight`)))

(event `RotateLeft`
  (bind (_minrotationz_roll _minrotationz_pitch _minrotationz_yaw) (`KismetMathLibrary.BreakRotator` (`self.MinRotationZ`)))
  (bind (_returnvalue_roll _returnvalue_pitch _returnvalue_yaw) (`KismetMathLibrary.BreakRotator` (`SceneComponent.K2_GetComponentRotation` (`self.DefaultSceneRoot`))))
  ;[1 1 1] Ballista Rotation
  (if (not (<= _returnvalue_yaw _minrotationz_yaw))
    (`/Engine/EditorBlueprintResources/StandardMacros.DoOnce` false :!label _label
      (:`Completed`
        (`self.K2_AddActorWorldRotation` (struct :`Yaw` -1.0))
        (goto _label :!via `Reset`)))))

(event `RotateRight`
  (bind (_maxrotationz_roll _maxrotationz_pitch _maxrotationz_yaw) (`KismetMathLibrary.BreakRotator` (`self.MaxRotationZ`)))
  (bind (_returnvalue_roll _returnvalue_pitch _returnvalue_yaw) (`KismetMathLibrary.BreakRotator` (`SceneComponent.K2_GetComponentRotation` (`self.DefaultSceneRoot`))))
  ;[1 1 1] Ballista Rotation
  (if (not (>= _returnvalue_yaw _maxrotationz_yaw))
    (`/Engine/EditorBlueprintResources/StandardMacros.DoOnce` false :!label _label_2
      (:`Completed`
        (`self.K2_AddActorWorldRotation` (struct :`Yaw` 1.0))
        (goto _label_2 :!via `Reset`)))))

(event `RotateUp`
  (bind _returnvalue (`self.GetTransform`))
  (bind (_returnvalue_roll _returnvalue_pitch) (`KismetMathLibrary.BreakRotator` (`self.K2_GetActorRotation`)))
  ;[1 1 1] Ballista Rotation
  (if (> _returnvalue_pitch 0.0)
    (`self.K2_SetActorTransform` (`KismetMathLibrary.MakeTransform` (.location _returnvalue) (`KismetMathLibrary.MakeRotator` (.roll (.rotation _returnvalue)) (- (.pitch (.rotation _returnvalue)) 1.0) (.yaw (.rotation _returnvalue))) (.scale _returnvalue)))))

(event `RotateDown`
  (bind _returnvalue (`self.GetTransform`))
  (bind (_returnvalue_roll _returnvalue_pitch) (`KismetMathLibrary.BreakRotator` (`self.K2_GetActorRotation`)))
  ;[1 1 1] Ballista Rotation
  (if (< _returnvalue_pitch 40.0)
    (`self.K2_SetActorTransform` (`KismetMathLibrary.MakeTransform` (.location _returnvalue) (`KismetMathLibrary.MakeRotator` (.roll (.rotation _returnvalue)) (+ (.pitch (.rotation _returnvalue)) 1.0) (.yaw (.rotation _returnvalue))) (.scale _returnvalue)))))

(event `Fire`
  ;[1 1 1] Firing
  (`/Engine/EditorBlueprintResources/StandardMacros.DoOnce` false :!label _label_3
    (:`Completed`
      (`GameplayStatics.PlaySound2D` "/Game/Audio/SFX/Ballista_Fire_Cue.Ballista_Fire_Cue" 1.0 1.0 0.0 null null)
      (bind _returnvalue (`|SpawnActorFromClass` "/Game/Objectives/Lvl2/BP_Projectile_Arrow.BP_Projectile_Arrow_C" (`SceneComponent.K2_GetComponentToWorld` (`self.ArrowSpawn`)) "Undefined" "OverrideRootScale" null null))
      (`PrimitiveComponent.AddImpulse` (`/Game/Objectives/Lvl2/BP_Projectile_Arrow.Arrow` _returnvalue) (* (`SceneComponent.GetForwardVector` (`self.ArrowSpawn`)) (`self.Cur Shot Force`)) "None" true)
      (`KismetSystemLibrary.Delay` 2.5)
      (goto _label_3 :!via `Reset`))))

(fn `UserConstructionScript`)