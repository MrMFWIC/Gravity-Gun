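; Level 2 barrier actor that removes itself once all three pedestal targets have been hit.
; A second after BeginPlay it caches the three target pedestals, finding each by class.
; Tick polls their TargetHit flags, and when all are true it plays an opening sound, waits briefly, then destroys the barrier.
; The sound call has no once-only guard, so it fires every frame during that wait.
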(event `self.ReceiveBeginPlay`
  (`KismetSystemLibrary.Delay` 1.0)
  (`self.Get Pedastal References`))

(event `Get Pedastal References`
  (bind _returnvalue (`GameplayStatics.GetActorOfClass` "/Game/Objectives/Lvl2/BP_Pedastal_C_Target1.BP_Pedastal_C_Target1_C"))
  (set `self.Target1` _returnvalue)
  (bind _returnvalue_2 (`GameplayStatics.GetActorOfClass` "/Game/Objectives/Lvl2/BP_Pedastal_C_Target2.BP_Pedastal_C_Target2_C"))
  (set `self.Target2` _returnvalue_2)
  (bind _returnvalue_3 (`GameplayStatics.GetActorOfClass` "/Game/Objectives/Lvl2/BP_Pedastal_C_Target3.BP_Pedastal_C_Target3_C"))
  (set `self.Target3` _returnvalue_3))

(event `self.ReceiveTick`
  (params (DeltaSeconds :type "Float (single-precision)"))
  (if (and (`/Game/Objectives/Lvl2/BP_Pedastal_C_Target1.TargetHit` (`self.Target1`)) (`/Game/Objectives/Lvl2/BP_Pedastal_C_Target2.TargetHit` (`self.Target2`)) (`/Game/Objectives/Lvl2/BP_Pedastal_C_Target3.TargetHit` (`self.Target3`)))
    (`GameplayStatics.PlaySound2D` "/Game/Audio/SFX/BarrierOpened.BarrierOpened" 0.5 1.0 0.0 null null)
    (`KismetSystemLibrary.Delay` 2.5)
    (`self.K2_DestroyActor`)))

(fn `UserConstructionScript`)